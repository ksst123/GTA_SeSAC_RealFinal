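; GTA-style player Blueprint that handles weapon switching through a pie menu.
; Triggering IA_WeaponTab creates a GTAPieMenu widget and switches to Game-and-UI input; releasing it only clears the open flag, as the widget removal code is unconnected.
; While the flag is set, IA_WeaponChange reads the menu selection and calls FightComponent's pistol or hand action, leaving the other two slots without actions.
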(event `EnhancedInput|/Game/Input/Actions/IA_WeaponChange`
  (params (ActionValue :type Boolean) (ElapsedSeconds :type "Float (double-precision)") (TriggeredSeconds :type "Float (double-precision)") (InputAction :type "InputAction Object Reference" :default "/Game/Input/Actions/IA_WeaponChange.IA_WeaponChange"))
  ;[1 1 1] WeaponChange
  (:`Triggered`
    (if (`self.WindowisOpen?`)
      (bind (_i1 _i2 _i3 _i4) (`/Game/UI/PieMenu/GTAPieMenu.CallSelection` (`self.PieMenuRef`)))
      (if _i2
        (`GTA_PlayerFightComponent.OnActionPistol` (`self.FightComponent`))
        (elif _i3
          _
          (elif _i1
            (`GTA_PlayerFightComponent.OnActionHand` (`self.FightComponent`))
            (elif _i4
              _)))))))

(event `EnhancedInput|/Game/Input/Actions/IA_WeaponTab`
  (params (ActionValue :type Boolean) (ElapsedSeconds :type "Float (double-precision)") (TriggeredSeconds :type "Float (double-precision)") (InputAction :type "InputAction Object Reference" :default "/Game/Input/Actions/IA_WeaponTab.IA_WeaponTab"))
  (bind _returnvalue (`GameplayStatics.GetPlayerController` 0))
  ;[1 1 1] PieMenu
  (:`Triggered`
    (set `self.WindowisOpen?` true)
    (bind _returnvalue_2 (`|CreateWidget` "/Game/UI/PieMenu/GTAPieMenu.GTAPieMenu_C"))
    (`/Game/UI/PieMenu/GTAPieMenu.StartSelection` _returnvalue_2)
    (bind _output_get (set `self.PieMenuRef` _returnvalue_2))
    (`UserWidget.AddToViewport` _output_get 0)
    (set `PlayerController.bShowMouseCursor` false _returnvalue)
    (`Controller.SetIgnoreLookInput` _returnvalue false)
    (`WidgetBlueprintLibrary.SetInputMode_GameAndUIEx` _returnvalue _output_get))
  (:`Completed`
    (set `self.WindowisOpen?` false)))

(fn `UserConstructionScript`)